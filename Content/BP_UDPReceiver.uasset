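; UDP receiver actor that, on non-HoloLens instances, discovers HoloLens clients from heartbeat messages on a broadcast socket.
; Tick polls the socket, relays each message through OnMsgReceved and extracts the ID after "HBID:".
; New IDs alternate between Hololens1 and Hololens2 by array index parity and are saved to MRGameInstance, which seeds the list on BeginPlay.
; A retriggerable delay clears the local client list once messages stop for a few seconds.
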(event `self.ReceiveBeginPlay`
  (`self.StartUDPReceiver` "bsApp" "255.255.255.255" 8182)
  (bind _asmrgame_instance (cast `/Game/BP/System/MRGameInstance` (`GameplayStatics.GetGameInstance`)))
  (set `self.isHololens` (`/Game/BP/System/MRGameInstance.IsHoloLens` _asmrgame_instance))
  (`KismetArrayLibrary.Array_Clear` (`self.Clients`))
  (bind _asmrgame_instance_2 (cast `/Game/BP/System/MRGameInstance` (`GameplayStatics.GetGameInstance`)))
  (set `self.Clients` (`/Game/BP/System/MRGameInstance.Clients` _asmrgame_instance_2)))

(event `self.ReceiveTick`
  (params (DeltaSeconds :type "Float (single-precision)"))
  (bind (_str _success) (`self.DataRecv`))
  (bind _clients (`self.Clients`))
  (bind (_lefts _rights) (`KismetStringLibrary.Split` _str "HBID:"))
  (if (`self.isHololens`)
    _
    (elif _success
      (`self.OnMsgReceved` _str)
      (if (not (`self.isHololens`))
        (`|ExecutionSequence`
          (:`then_0`
            (`KismetSystemLibrary.RetriggerableDelay` 5.0)
            (`KismetArrayLibrary.Array_Clear` (`self.Clients`)))
          (:`then_1`
            (if (not (`KismetArrayLibrary.Array_Contains` _clients _rights))
              (bind _returnvalue (`KismetArrayLibrary.Array_AddUnique` _clients _rights))
              (switch `int` (mod _returnvalue 2)
                (:`0`
                  (bind _output_get (set `/Game/LANTools/BP_Hololens.Client` _rights (`self.Hololens1`)))
                  (bind _asmrgame_instance (cast `/Game/BP/System/MRGameInstance` (`GameplayStatics.GetGameInstance`)))
                  (set `/Game/BP/System/MRGameInstance.Hololens1Client` _output_get _asmrgame_instance)
                  (set `/Game/BP/System/MRGameInstance.Clients` _clients _asmrgame_instance))
                (:`1`
                  (bind _output_get_2 (set `/Game/LANTools/BP_Hololens.Client` _rights (`self.Hololens2`)))
                  (bind _asmrgame_instance_2 (cast `/Game/BP/System/MRGameInstance` (`GameplayStatics.GetGameInstance`)))
                  (set `/Game/BP/System/MRGameInstance.Hololens2Client` _output_get_2 _asmrgame_instance_2)
                  (set `/Game/BP/System/MRGameInstance.Clients` _clients _asmrgame_instance_2))))))))))

(fn `UserConstructionScript`)