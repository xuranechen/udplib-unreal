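; BP_UDPSender is a UDP broadcast sender that announces a HoloLens device on the local network and sends text messages.
; BeginPlay opens a Rama UDP socket to the broadcast address, generates a GUID and reads the HoloLens flag from MRGameInstance.
; On HoloLens, it sends that ID as a heartbeat immediately and then on a looping timer.
; SendText transmits only on HoloLens, while SendMSG sends on any device.
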(event `self.ReceiveBeginPlay`
  (`self.StartUDPSender` "bsApp" "255.255.255.255" 8182 true)
  (set `self.ID` (`KismetGuidLibrary.Conv_GuidToString` (`KismetGuidLibrary.NewGuid`)))
  (bind _asmrgame_instance (cast `/Game/BP/System/MRGameInstance` (`GameplayStatics.GetGameInstance`)))
  (bind _output_get (set `self.isHololens` (`/Game/BP/System/MRGameInstance.IsHoloLens` _asmrgame_instance)))
  (set `self.As MRGame Instance` _asmrgame_instance)
  (if _output_get
    (`KismetSystemLibrary.K2_SetTimerDelegate` (delegate `SendHeartbeat`) 2.0 true)
    (`self.SendText` (`KismetStringLibrary.Concat_StrStr` "HBID:" (`self.ID`)) :!label _label)))

(event `SendHeartbeat`
  (goto _label))

(event `SendText`
  (params (Text :type String))
  (if (`self.isHololens`)
    (`self.RamaUDPSender_SendString` Text)))

(event `SendMSG`
  (params (ToSend :type String))
  (`self.RamaUDPSender_SendString` ToSend))

(fn `UserConstructionScript`)